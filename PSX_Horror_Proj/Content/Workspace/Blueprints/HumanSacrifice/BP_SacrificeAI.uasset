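; BP_SacrificeAI is an AI pawn that patrols a looping route of waypoint actors.
; On BeginPlay it stores the waypoint count and starts FollowWaypoint, which uses AIMoveTo to walk the pawn to the current waypoint.
; Each successful move advances the index, wraps to the first at the end, and calls FollowWaypoint again after a short delay.
; A failed move has no handler, so the patrol stops there.
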(event `self.ReceiveBeginPlay`
  (set `self.MaxWaypoints` (`KismetArrayLibrary.Array_Length` (`self.Waypoints`)))
  (`self.Follow waypoint`))

(event `Follow waypoint`
  (bind _currentwaypoint (`self.CurrentWaypoint`))
  (`|AIMoveTo` self (0.0 0.0 0.0) (`|GetArrayItem` (`self.Waypoints`) (`self.CurrentWaypoint`))
    (:`OnSuccess`
      (`/Engine/EditorBlueprintResources/StandardMacros.IncrementInt` _currentwaypoint
        (:`  `
          (if (>= _currentwaypoint (`self.MaxWaypoints`))
            (set `self.CurrentWaypoint` 0))
          (`KismetSystemLibrary.Delay` 0.2)
          (`self.Follow waypoint`))))))

(fn `UserConstructionScript`)